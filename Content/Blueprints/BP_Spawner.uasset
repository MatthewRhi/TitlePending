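; Rhythm note spawner that turns a hand of cards into moving BP_Note actors when the action phase begins.
; Player controller events trigger spawning and increment a missed-note counter, which resets as cards spawn.
; All notes spawn at once, spaced along Y by note offset plus one bar per card.
; A shared local-space projectile velocity sets the tempo, turning distance into timing.
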(event `self.ReceiveBeginPlay`
  ;[1 1 1] Represents bar length (1000 units = 1 bar) (-500Y = 120bpm)
  (set `self.CardOffset` 1000.0)
  (set `self.SpawnVelocity` (0.0 -500.0 0.0))
  (bind _asbp_gameplay_phase_player_controller (cast `/Game/Blueprints/BP_GameplayPhase_PlayerController` (`GameplayStatics.GetPlayerController` 0)))
  (add `/Game/Blueprints/BP_GameplayPhase_PlayerController.OnNoteMissed` _asbp_gameplay_phase_player_controller (delegate `IncrementNotesMissed`))
  (add `/Game/Blueprints/BP_GameplayPhase_PlayerController.BeginActionPhase` _asbp_gameplay_phase_player_controller (delegate `OnBeginActionPhase`)))

(event `IncrementNotesMissed`
  (params (Card :type "/Game/Blueprints/DataTables/F_CardStructure Structure") (Name :type Name))
  (`/Engine/EditorBlueprintResources/StandardMacros.IncrementInt` (`self.NotesMissed`)))

(event `OnBeginActionPhase`
  (params (Hand :type "Array of /Game/Blueprints/DataTables/F_CardStructure Structure (by ref)"))
  (`self.SpawnCardsFromHand` Hand))

(fn `Spawn`
  (params (NoteType :type String) (Offset :type "Float (double-precision)"))
  (bind (_returnvalue_location _returnvalue_rotation) (`KismetMathLibrary.BreakTransform` (`self.GetTransform`)))
  (bind _returnvalue (`|SpawnActorFromClass` "/Game/Blueprints/BP_Note.BP_Note_C" (`KismetMathLibrary.MakeTransform` (+ _returnvalue_location (`KismetMathLibrary.MakeVector` 0.0 Offset)) _returnvalue_rotation (`self.SpawnScale`)) "Undefined" "OverrideRootScale" null NoteType (`self.CurrentCard`) null))
  (`/Game/Blueprints/BP_Note.DisplayType` _returnvalue)
  (`ProjectileMovementComponent.SetVelocityInLocalSpace` (`/Game/Blueprints/BP_Note.ProjectileMovement` _returnvalue) (`self.SpawnVelocity`)))

(fn `SpawnCardsFromHand`
  (params (Hand :type "Array of /Game/Blueprints/DataTables/F_CardStructure Structure"))
  (for (_array_element _array_index) Hand
    (bind _output_get (set `self.CurrentCard` _array_element))
    (set `self.NotesMissed` 0)
    (`self.SpawnNotesFromCard` (`.Notes_43_E2D9BC2C4091FD2748348EA87304AACA` (break `/Game/Blueprints/DataTables/F_CardStructure` _output_get)) (`.Offset_28_733363A747BA322D47F7DEA0ED58D10A` (break `/Game/Blueprints/DataTables/F_CardStructure` _output_get)) (* _array_index (`self.CardOffset`)))))

(fn `SpawnNotesFromCard`
  (params (Notes :type "Array of String") (Offsets :type "Array of Float (double-precision)") (CardOffset :type "Float (double-precision)"))
  ;[1 1 1] This function exists purlely to allow for loops during testing
  (for (_array_element _array_index) Notes
    (`self.Spawn` _array_element (+ (`|GetArrayItem` Offsets _array_index) CardOffset))))

(fn `UserConstructionScript`)