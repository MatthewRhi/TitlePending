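; Player controller for a rhythm card battler that alternates between a planning phase, where the hand is shown, and an action phase, where cards resolve through notes.
; It builds the hand from the player's deck via a data table and swaps phase widgets using event dispatchers.
; Each card's hit-note ratio sets a three-tier execution score that scales its damage, armor or healing.
; The turn ends after the last card, and zero health loads the lose screen.
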(event `self.ReceiveBeginPlay`
  (bind _hand (`self.InitializeBeginningDeck`))
  (bind _returnvalue (`|CreateWidget` "/Game/Blueprints/Widgets/WBP_PlayerHand.WBP_PlayerHand_C" null _hand))
  (bind _output_get (set `self.PlanningPhaseUI` _returnvalue))
  (`UserWidget.AddToViewport` _output_get 0)
  (bind _aswbp_player_hand (cast `/Game/Blueprints/Widgets/WBP_PlayerHand` _output_get))
  (`self.ToPlanningPhase` (`self.Hand`))
  (add `/Game/Blueprints/Widgets/WBP_PlayerHand.SwitchToActionPhase` _aswbp_player_hand (delegate `OnSwitchToActionPhase`))
  ;[1 1 1] Action Phase
  (`self.InitializeUIVars`)
  ;;[1 1 1] Note Events and Handling
  (add `Button.OnPressed` (`self.LeftBtn`) (delegate `LeftBtnPressed`))
  (add `Button.OnPressed` (`self.RightBtn`) (delegate `RightBtnPressed`))
  (add `self.OnNotePlayed` (delegate `NotePlayed`))
  (add `self.OnNoteMissed` (delegate `NoteMissed`))
  ;;[1 1 1] Card Events and Handling
  (add `self.CardChanged` (delegate `OnCardChanged`))
  (add `self.OnExecutionDetermined` (delegate `CardEffect`))
  (add `self.PlayerDamaged` (delegate `OnPlayerDamaged`))
  ;;[255 -0.9481 1] Bind End Of Turn Stuff
  (add `self.EndOfTurn` (delegate `OnEndOfTurn`)))

(event `LeftBtnPressed`
  ;[1 1 1] Action Phase
  ;;[1 1 1] Note Events and Handling
  (`self.OnLeftBtnPressed`))

(event `RightBtnPressed`
  ;[1 1 1] Action Phase
  ;;[1 1 1] Note Events and Handling
  (`self.OnRightBtnPressed`))

(event `NotePlayed` :!signature `self.OnNotePlayed`
  (params (Card :type "/Game/Blueprints/DataTables/F_CardStructure Structure") (Name :type Name))
  ;[1 1 1] Action Phase
  ;;[1 1 1] Note Events and Handling
  (`self.HandleNoteEvents` Card)
  (`self.ShowPopup` true)
  (`self.NoteCorrectAnimation`))

(event `NoteMissed` :!signature `self.OnNoteMissed`
  (params (Card :type "/Game/Blueprints/DataTables/F_CardStructure Structure") (Name :type Name))
  ;[1 1 1] Action Phase
  ;;[1 1 1] Note Events and Handling
  (`self.HandleNoteEvents` Card true)
  (`self.ShowPopup` false))

(event `OnCardChanged`
  ;[1 1 1] Action Phase
  ;;[1 1 1] Card Events and Handling
  (`self.HandleCardChanged` (`self.PlayerUI`)))

(event `OnPlayerDamaged` :!signature `self.PlayerDamaged`
  (params (Damage :type Integer))
  ;[1 1 1] Action Phase
  ;;[1 1 1] Card Events and Handling
  (`self.DamagePlayer` Damage))

(event `OnEndOfTurn`
  ;[1 1 1] Action Phase
  ;;[255 -0.9481 1] Bind End Of Turn Stuff
  (`KismetSystemLibrary.Delay` 0.25)
  (`self.SwitchToPlanningPhase`)
  (`self.ToPlanningPhase` (`self.Hand`))
  (`self.SwitchTrack`))

(event `CardEffect` :!signature `self.OnExecutionDetermined`
  (params (PercentageCorrect :type "Float (double-precision)") (ExecutionScore :type Integer) (Card :type "/Game/Blueprints/DataTables/F_CardStructure Structure") (PlayerUI :type "/Game/Blueprints/Widgets/WBP_ActionPhase_PlayerInterface Object Reference"))
  ;[1 1 1] Action Phase
  ;;[1 1 1] Card Events and Handling
  (`self.ApplyCardEffect` Card ExecutionScore)
  (`self.PlayerTurnTaken`)
  (`self.EndOfTurnCalculator`))

(event `OnSwitchToActionPhase`
  (params (Hand :type "Array of /Game/Blueprints/DataTables/F_CardStructure Structure (by ref)"))
  (`self.SwitchToActionPhase` Hand)
  ;[1 1 1] Action Phase
  (`self.SwitchTrack`))

(fn `ApplyCardEffect`
  (params (Card :type "/Game/Blueprints/DataTables/F_CardStructure Structure") (Execution :type Integer))
  (bind _returnvalue (subsystem `PlayerStats`))
  (`KismetSystemLibrary.PrintString` (`KismetStringLibrary.Concat_StrStr` "Card Type:" Card_Type_8_1E0703B94F02174D5996068830E6116F "Execution Score" (`KismetStringLibrary.Conv_IntToString` Execution) "Max Value" (`KismetStringLibrary.Conv_IntToString` Card_ValueSuccess_21_0842977347F5FD1895A8FBA131177635)))
  (switch `string` Card_Type_8_1E0703B94F02174D5996068830E6116F
    (:`Attack`
      (switch `int` Execution
        (:`0`
          (`self.DamageEnemy` Card_ValueFail_20_CABB3F4B4FC198DE2BA164B02552AB06))
        (:`1`
          (`self.DamageEnemy` Card_ValuePartial_18_C461449146934529E91B5580F26020A8))
        (:`2`
          (`self.DamageEnemy` Card_ValueSuccess_21_0842977347F5FD1895A8FBA131177635))))
    (:`Defense`
      (switch `int` Execution
        (:`0`
          (`PlayerStats.AddArmor` _returnvalue Card_ValueFail_20_CABB3F4B4FC198DE2BA164B02552AB06))
        (:`1`
          (`PlayerStats.AddArmor` _returnvalue Card_ValuePartial_18_C461449146934529E91B5580F26020A8))
        (:`2`
          (`PlayerStats.AddArmor` _returnvalue Card_ValueSuccess_21_0842977347F5FD1895A8FBA131177635))))
    (:`Utility`
      (switch `int` Execution
        (:`0`
          (`PlayerStats.HealDamage` _returnvalue Card_ValueFail_20_CABB3F4B4FC198DE2BA164B02552AB06))
        (:`1`
          (`PlayerStats.HealDamage` _returnvalue Card_ValuePartial_18_C461449146934529E91B5580F26020A8))
        (:`2`
          (`PlayerStats.HealDamage` _returnvalue Card_ValueSuccess_21_0842977347F5FD1895A8FBA131177635))))))

(fn `CardSwipe`
  (bind _playerui (`self.PlayerUI`))
  (`UserWidget.PlayAnimation` _playerui (`/Game/Blueprints/Widgets/WBP_ActionPhase_PlayerInterface.Swipe` _playerui) 0.0 1 "Forward" 0.8 false))

(fn `ClearPopup`
  (`Widget.RemoveFromParent` (`self.CurrentPopup`)))

(fn `DamagePlayer`
  (params (Damage :type Integer))
  (bind _returnvalue (subsystem `PlayerStats`))
  (bind _playerui (`self.PlayerUI`))
  (`UserWidget.PlayAnimation` _playerui (`/Game/Blueprints/Widgets/WBP_ActionPhase_PlayerInterface.HurtAnimation` _playerui) 0.0 1 "Forward" 1.0 false)
  (`PlayerStats.TakeDamage` _returnvalue Damage)
  (if (<= (`PlayerStats.CurrentHealth` _returnvalue) 0)
    (`GameplayStatics.OpenLevel` "LoseScreen")))

(fn `DetermineLastNote`
  (bind (_currentcard_name _currentcard_type _currentcard_valuefail _currentcard_valuepartial _currentcard_valuesuccess _currentcard_notes) (break `/Game/Blueprints/DataTables/F_CardStructure` (`self.CurrentCard`)))
  (bind _result (`/Engine/EditorBlueprintResources/StandardMacros.IncrementInt` (`self.Notes`))
    (:`  `
      (if (== _result (`KismetArrayLibrary.Array_Length` _currentcard_notes))
        (`self.GetPercentageCorrect`)))))

(fn `EndOfTurnCalculator`
  (bind _result (`/Engine/EditorBlueprintResources/StandardMacros.IncrementInt` (`self.NumberofCardsPlayed`))
    (:`  `
      (if (>= _result (`KismetArrayLibrary.Array_Length` (`self.Hand`)))
        (`self.EndOfTurn`)))))

(fn `EnemyAction`
  (bind _targetedenemy (`self.TargetedEnemy`))
  (for _ (range 5)
    (`KismetArrayLibrary.Array_Add` (`self.EnemyActionType`) (`KismetMathLibrary.RandomInteger` 3))
    (`KismetSystemLibrary.PrintString` "AddedElement"))
  (for _array_element (`self.EnemyActionType`)
    (if (== _array_element 1)
      (`self.DamagePlayer` 0)
      (else
        (set `/Game/Blueprints/BP_EnemyIcon.Armor` (+ (`/Game/Blueprints/BP_EnemyIcon.Armor` _targetedenemy) (`/Game/Blueprints/BP_EnemyIcon.Defense` _targetedenemy)) _targetedenemy)))))

(fn `GetNextCard`
  (returns (NextCard :type "/Game/Blueprints/DataTables/F_CardStructure Structure (by ref)") (ReturnValue :type Boolean))
  (bind _hand (`self.Hand`))
  (bind _numberofcardsplayed (`self.NumberofCardsPlayed`))
  (bind _returnvalue (`KismetArrayLibrary.Array_IsValidIndex` _hand _numberofcardsplayed))
  (if _returnvalue
    (return (`|GetArrayItem` _hand _numberofcardsplayed) _returnvalue)
    (else
      (return (struct) _returnvalue))))

(fn `GetPercentageCorrect`
  (returns (PercentageCorrect :type "Float (double-precision)") (ExecutionScore :type Integer))
  (bind (_currentcard_name _currentcard_type _currentcard_valuefail _currentcard_valuepartial _currentcard_valuesuccess _currentcard_notes) (break `/Game/Blueprints/DataTables/F_CardStructure` (`self.CurrentCard`)))
  (bind _returnvalue (`KismetArrayLibrary.Array_Length` _currentcard_notes))
  (bind _returnvalue_2 (/ (`KismetMathLibrary.Conv_IntToDouble` (- _returnvalue (`self.NotesMissed`))) (`KismetMathLibrary.Conv_IntToDouble` _returnvalue)))
  (if (`KismetMathLibrary.InRange_FloatFloat` _returnvalue_2 0.0 0.5 true false)
    (return _returnvalue_2 0)
    (elif (`KismetMathLibrary.InRange_FloatFloat` _returnvalue_2 0.5 0.75 true false)
      (return _returnvalue_2 1)
      (else
        (return _returnvalue_2 2)))))

(fn `HandleCardChanged`
  (params (UI :type "/Game/Blueprints/Widgets/WBP_ActionPhase_PlayerInterface Object Reference"))
  (bind _currentcardbox (`/Game/Blueprints/Widgets/WBP_ActionPhase_PlayerInterface.CurrentCardBox` UI))
  (`PanelWidget.ClearChildren` _currentcardbox)
  (`self.CardSwipe`)
  (bind (_nextcard _returnvalue) (`self.GetNextCard`))
  (if _returnvalue
    (bind _returnvalue_2 (`|CreateWidget` "/Game/Blueprints/Widgets/WBP_Card.WBP_Card_C" (`GameplayStatics.GetPlayerController` 0) _nextcard))
    (`/Game/Blueprints/Widgets/WBP_Card.DisplayCard` _returnvalue_2)
    (bind _returnvalue_3 (`Overlay.AddChildToOverlay` _currentcardbox _returnvalue_2))
    (`OverlaySlot.SetHorizontalAlignment` _returnvalue_3 "HAlign_Fill")
    (`OverlaySlot.SetVerticalAlignment` _returnvalue_3 "VAlign_Fill")))

(fn `HandleNoteEvents`
  (params (Card :type "/Game/Blueprints/DataTables/F_CardStructure Structure") (NoteMissed :type Boolean))
  (locals (NoteIsMissed :type Boolean) (PotentialCard :type "/Game/Blueprints/DataTables/F_CardStructure Structure"))
  (bind _output_get (set `self.CurrentCard` Card))
  (set `local.NoteIsMissed` NoteMissed)
  (`/Engine/EditorBlueprintResources/StandardMacros.IncrementInt` (`self.Notes`)
    (:`  `
      (set `self.NotesMissed` (+ (`self.NotesMissed`) (`KismetMathLibrary.Conv_BoolToInt` (`local.NoteIsMissed`))))
      (if (== (`self.Notes`) (`KismetArrayLibrary.Array_Length` (`.Notes_43_E2D9BC2C4091FD2748348EA87304AACA` (break `/Game/Blueprints/DataTables/F_CardStructure` _output_get))))
        (bind (_percentagecorrect _executionscore) (`self.GetPercentageCorrect`))
        (`self.OnExecutionDetermined` _percentagecorrect _executionscore (`self.CurrentCard`) (`self.PlayerUI`))
        (set `self.Notes` 0)
        (set `self.NotesMissed` 0)
        (set `self.CardShouldChange` true)
        (`self.CardChanged`)
        (else
          (set `self.CardShouldChange` false))))))

(fn `InitializeBeginningDeck`
  (returns (Hand :type "Array of /Game/Blueprints/DataTables/F_CardStructure Structure"))
  (bind _returnvalue (subsystem `PlayerStats`))
  (if (<= (`KismetArrayLibrary.Array_Length` (`PlayerStats.playerDeck` (subsystem `PlayerStats`))) 0)
    (`PlayerStats.ObliterateDeck` _returnvalue)
    (`PlayerStats.InitializeDeck` _returnvalue))
  (`KismetArrayLibrary.Array_Clear` (`self.Hand`))
  (for _array_element (`PlayerStats.playerDeck` (subsystem `PlayerStats`))
    (bind _returnvalue_2 (`|GetDataTableRow` "/Game/Blueprints/DataTables/DT_CardTable.DT_CardTable" _array_element)
      (:`then`
        (`KismetArrayLibrary.Array_Add` (`self.Hand`) _returnvalue_2))
      (:`RowNotFound`
        (`KismetSystemLibrary.PrintString` "Row not found when adding card to hand"))))
  (return (`self.Hand`)))

(fn `InitializeHealthBars`
  (bind _returnvalue (`|CreateWidget` "/Game/Blueprints/Widgets/WBP_StatsHUD.WBP_StatsHUD_C"))
  (bind _output_get (set `self.PlayerStatsUI` _returnvalue))
  (`UserWidget.AddToViewport` _output_get 0))

(fn `InitializeUIVars`
  (bind _returnvalue (`|CreateWidget` "/Game/Blueprints/Widgets/WBP_ActionPhase_PlayerInterface.WBP_ActionPhase_PlayerInterface_C"))
  (bind _output_get (set `self.PlayerUI` _returnvalue))
  (set `self.LeftBtn` (`/Game/Blueprints/Widgets/WBP_ActionPhase_PlayerInterface.LeftBtn` _output_get))
  (set `self.RightBtn` (`/Game/Blueprints/Widgets/WBP_ActionPhase_PlayerInterface.RightBtn` _output_get)))

(fn `NoteCorrectAnimation`
  (bind _playerui (`self.PlayerUI`))
  (`UserWidget.PlayAnimation` _playerui (`/Game/Blueprints/Widgets/WBP_ActionPhase_PlayerInterface.CardWiggle` _playerui) 0.0 1 "Forward" 1.0 false))

(fn `ShowPopup`
  (params (doesHit :type Boolean))
  (if doesHit
    (`KismetSystemLibrary.K2_SetTimer` null "ClearPopup" 0.5)
    (bind _returnvalue (`|CreateWidget` "/Game/Blueprints/Widgets/WBP_PopupHit.WBP_PopupHit_C" (`GameplayStatics.GetPlayerController` 0)))
    (`UserWidget.AddToViewport` _returnvalue 0)
    (set `self.CurrentPopup` _returnvalue)
    (else
      (`KismetSystemLibrary.K2_SetTimer` null "ClearPopup" 0.5)
      (bind _returnvalue_2 (`|CreateWidget` "/Game/Blueprints/Widgets/WBP_PopupMiss.WBP_PopupMiss_C" (`GameplayStatics.GetPlayerController` 0)))
      (`UserWidget.AddToViewport` _returnvalue_2 0)
      (set `self.CurrentPopup` _returnvalue_2))))

(fn `SwitchToActionPhase`
  (params (Hand :type "Array of /Game/Blueprints/DataTables/F_CardStructure Structure (by ref)"))
  (bind _output_get (set `self.CurrentCard` (`|GetArrayItem` Hand)))
  (set `self.NumberofCardsPlayed` 0)
  (bind _returnvalue (`|CreateWidget` "/Game/Blueprints/Widgets/WBP_Card.WBP_Card_C" (`GameplayStatics.GetPlayerController` 0) _output_get))
  (`/Game/Blueprints/Widgets/WBP_Card.DisplayCard` _returnvalue)
  (bind _returnvalue_2 (`Overlay.AddChildToOverlay` (`/Game/Blueprints/Widgets/WBP_ActionPhase_PlayerInterface.CurrentCardBox` (`self.PlayerUI`)) _returnvalue))
  (`OverlaySlot.SetHorizontalAlignment` _returnvalue_2 "HAlign_Fill")
  (`OverlaySlot.SetVerticalAlignment` _returnvalue_2 "VAlign_Fill")
  (`Widget.RemoveFromParent` (`self.PlanningPhaseUI`))
  (`UserWidget.AddToViewport` (`self.PlayerUI`) 0)
  (`self.InitializeHealthBars`)
  (`self.BeginActionPhase` Hand))

(fn `SwitchToPlanningPhase`
  (bind _planningphaseui (`self.PlanningPhaseUI`))
  (set `self.NumberofCardsPlayed` 0)
  (`Widget.RemoveFromParent` (`self.PlayerStatsUI`))
  (`Widget.RemoveFromParent` (`self.PlayerUI`))
  (`/Game/Blueprints/Widgets/WBP_PlayerHand.ClearPlayingOrder` _planningphaseui)
  (`UserWidget.AddToViewport` _planningphaseui 0)
  (set `self.CurrentCard` (struct)))

(fn `UserConstructionScript`)