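; BP_GoodZone is a hit zone for notes, judging left and right button presses in the gameplay phase.
; Its Cube overlap stores the entering BP_Note and toggles that note's Destructible flag on entry and exit.
; Button events bound from the gameplay PlayerController pass "L" or "R" to the stored note's EvaluateExpectation.
; Only the last entered note is tracked, and the reference is not cleared on exit.
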(event `self.ReceiveBeginPlay`
  (bind _asbp_gameplay_phase_player_controller (cast `/Game/Blueprints/BP_GameplayPhase_PlayerController` (`GameplayStatics.GetPlayerController` 0)))
  (set `self.PlayerController` _asbp_gameplay_phase_player_controller)
  (add `/Game/Blueprints/BP_GameplayPhase_PlayerController.OnLeftBtnPressed` (`self.PlayerController`) (delegate `HandleLeftBtn`))
  (add `/Game/Blueprints/BP_GameplayPhase_PlayerController.OnRightBtnPressed` (`self.PlayerController`) (delegate `HandleRightBtn`)))

(event `HandleLeftBtn`
  (`self.HandleButtonInput` "L"))

(event `HandleRightBtn`
  (`self.HandleButtonInput` "R"))

(event `self.Cube.OnComponentBeginOverlap`
  (params (OverlappedComponent :type "PrimitiveComponent Object Reference") (OtherActor :type "Actor Object Reference") (OtherComp :type "PrimitiveComponent Object Reference") (OtherBodyIndex :type Integer) (bFromSweep :type Boolean) (SweepResult :type "HitResult Structure (by ref)"))
  (bind _asbp_note (cast `/Game/Blueprints/BP_Note` OtherActor))
  (set `self.Note` _asbp_note)
  (set `/Game/Blueprints/BP_Note.Destructible` true _asbp_note))

(event `self.Cube.OnComponentEndOverlap`
  (params (OverlappedComponent :type "PrimitiveComponent Object Reference") (OtherActor :type "Actor Object Reference") (OtherComp :type "PrimitiveComponent Object Reference") (OtherBodyIndex :type Integer))
  (bind _asbp_note (cast `/Game/Blueprints/BP_Note` OtherActor))
  (set `/Game/Blueprints/BP_Note.Destructible` false _asbp_note))

(fn `CallNotePlayed`
  (`/Game/Blueprints/BP_GameplayPhase_PlayerController.OnNotePlayed` (`self.PlayerController`) (`self.CurrentCard`) "None")
  (set `self.LeftRecieved` false)
  (set `self.RightRecieved` false)
  (`self.K2_DestroyActor` (`self.NoteInPlayzone`)))

(fn `HandleButtonInput`
  (params (Side :type String))
  (bind _note (`self.Note`))
  (if (`KismetSystemLibrary.IsValid` _note)
    (`/Game/Blueprints/BP_Note.EvaluateExpectation` _note Side)))

(fn `Print`
  (params (NoteType :type String) (Box :type String))
  (`KismetSystemLibrary.PrintString` (`KismetStringLibrary.Concat_StrStr` NoteType " in" Box)))

(fn `UserConstructionScript`)