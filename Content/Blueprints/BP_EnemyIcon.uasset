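; Enemy in a turn-based card battle, with a random DT_EnemyInfo row supplying its stats, flipbooks and possible actions.
; Player controller events drive it: planning queues up to five random actions as widget icons, and each player turn consumes one to attack, block or heal.
; Incoming damage is reduced by armor, and death opens the win screen.
; A select-based animation state swaps flipbooks, with timers restoring idle.
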(event `self.ReceiveBeginPlay`
  (`self.InitializeEnemy`)
  (bind _asbp_gameplay_phase_player_controller (cast `/Game/Blueprints/BP_GameplayPhase_PlayerController` (`GameplayStatics.GetPlayerController` 0)))
  (add `/Game/Blueprints/BP_GameplayPhase_PlayerController.PlayerTurnTaken` _asbp_gameplay_phase_player_controller (delegate `OnPlayerTurnTaken`))
  (add `/Game/Blueprints/BP_GameplayPhase_PlayerController.DamageEnemy` _asbp_gameplay_phase_player_controller (delegate `OnEnemyDamaged`))
  (add `/Game/Blueprints/BP_GameplayPhase_PlayerController.ToPlanningPhase` _asbp_gameplay_phase_player_controller (delegate `OnToPlanningPhase`)))

(event `OnPlayerTurnTaken`
  (bind _enemysprite (`self.EnemySprite`))
  (`self.TakeEnemyTurn`)
  (bind _paperflipbook (`self.AnimStateMachine`))
  (`PaperFlipbookComponent.SetFlipbook` _enemysprite _paperflipbook)
  (`KismetSystemLibrary.K2_SetTimer` null "ResetAnimation" (`PaperFlipbookComponent.GetFlipbookLength` _enemysprite)))

(event `OnEnemyDamaged`
  (params (Damage :type Integer))
  (bind _enemydead (`self.DamageEnemy` Damage))
  (bind _paperflipbook (`self.AnimStateMachine`))
  (`PaperFlipbookComponent.SetFlipbook` (`self.EnemySprite`) _paperflipbook)
  (if _enemydead
    (set `self.EnemyTakeAction` false)
    (bind _asbp_gameplay_phase_player_controller (cast `/Game/Blueprints/BP_GameplayPhase_PlayerController` (`GameplayStatics.GetPlayerController` 0)))
    (`/Game/Blueprints/BP_GameplayPhase_PlayerController.EnemyDead` _asbp_gameplay_phase_player_controller)
    (`KismetSystemLibrary.Delay` 1.0)
    (`GameplayStatics.OpenLevel` "WinScreen")))

(event `OnToPlanningPhase`
  (params (Hand :type "Array of /Game/Blueprints/DataTables/F_CardStructure Structure (by ref)"))
  (`self.DetermineEnemyTurn` (`KismetMathLibrary.Min` (`KismetArrayLibrary.Array_Length` Hand) 5))
  (set `self.TurnCount` 0))

(fn `AnimStateMachine`
  (returns (PaperFlipbook :type "PaperFlipbook Object Reference"))
  (if (`self.EnemyTakeAction`)
    (set `self.EnemyTakeAction` false)
    (elif (<= (`self.CurrentHealth`) 0)
      (set `self.AnimationState` "NewEnumerator2")
      (else
        ;[1 1 1] Timer for resetting to idle animation after damaged animation is called
        (`KismetSystemLibrary.K2_SetTimer` null "ResetAnimation" 0.5)
        (set `self.AnimationState` "NewEnumerator0"))))
  (return (select `/Game/Sprites/Slime/AnimationState` (`self.AnimationState`) :`NewEnumerator0` (`self.IdleFlipbook`) :`NewEnumerator2` (`self.DeathFlipbook`) :`NewEnumerator3` (`self.AttackFlipbook`) :`NewEnumerator4` (`self.BlockFlipbook`) :`NewEnumerator5` (`self.HealFlipbook`))))

(fn `ApplyCardEffect`
  (params (Card :type String))
  (locals (CardName :type String) (CardValue :type Integer) (CardFound :type Boolean :default false) (PlayerController :type "/Game/Blueprints/BP_GameplayPhase_PlayerController Object Reference"))
  (bind _cardfound (`local.CardFound`))
  (bind (_value _returnvalue) (`BlueprintMapLibrary.Map_Find` (`self.Actions`) (`local.CardName`)))
  (set `local.CardName` Card)
  (bind _asbp_gameplay_phase_player_controller (cast `/Game/Blueprints/BP_GameplayPhase_PlayerController` (`GameplayStatics.GetPlayerController` 0)))
  (set `local.PlayerController` _asbp_gameplay_phase_player_controller)
  (set `local.CardValue` _value)
  (set `local.CardFound` _returnvalue)
  (switch `string` (`local.CardName`)
    (:`Attack`
      (if _cardfound
        (`KismetSystemLibrary.PrintString` "Attacking Player")
        (set `self.AnimationState` "NewEnumerator3")
        (`/Game/Blueprints/BP_GameplayPhase_PlayerController.PlayerDamaged` (`local.PlayerController`) (`local.CardValue`))
        (else
          (`KismetSystemLibrary.PrintString` "Failed to attack player"))))
    (:`Block`
      (if _cardfound
        (bind _output_get (set `self.Armor` (+ (stale _output_get) (`local.CardValue`))))
        (`KismetSystemLibrary.PrintString` "Enemy Blocking")
        (set `self.AnimationState` "NewEnumerator4")
        (else
          (`KismetSystemLibrary.PrintString` "Failed to block"))))
    (:`Heal`
      (if _cardfound
        (bind _returnvalue_2 (+ (stale _output_get_2) (`local.CardValue`)))
        (bind _output_get_2 (set `self.CurrentHealth` _returnvalue_2))
        (`KismetSystemLibrary.PrintString` "Enemy Healing")
        (if (>= _returnvalue_2 (`self.MaxHealth`))
          (set `self.CurrentHealth` (`self.MaxHealth`))
          (set `self.AnimationState` "NewEnumerator5"))
        (else
          (`KismetSystemLibrary.PrintString` "Failed to heal"))))))

(fn `DamageEnemy`
  (params (Damage :type Integer))
  (returns (EnemyDead :type Boolean))
  (locals (maxDamage :type Integer :default 0))
  (set `local.maxDamage` (- Damage (`self.Armor`)))
  (set `self.Armor` (`KismetMathLibrary.Max` (- (`self.Armor`) Damage)))
  (if (> (`local.maxDamage`) 0)
    (bind _output_get (set `self.CurrentHealth` (`KismetMathLibrary.Max` (- (`self.CurrentHealth`) (`local.maxDamage`)))))
    (return (<= _output_get 0))))

(fn `DetermineEnemyTurn`
  (params (Length :type Integer))
  (bind _aswbp_enemy_actions (cast `/Game/Blueprints/Widgets/WBP_EnemyActions` (`WidgetComponent.GetUserWidgetObject` (`self.Widget`))))
  (`KismetArrayLibrary.Array_Clear` (`PanelWidget.GetAllChildren` (`/Game/Blueprints/Widgets/WBP_EnemyActions.Actions` _aswbp_enemy_actions)))
  (bind _keys (`BlueprintMapLibrary.Map_Keys` (`self.Actions`)))
  (`KismetArrayLibrary.Array_Clear` (`self.ActionsForTurn`))
  (for _ (range Length)
    (`KismetArrayLibrary.Array_Add` (`self.ActionsForTurn`) (`|GetArrayItem` _keys (`KismetMathLibrary.RandomIntegerInRange` 0 (- (`KismetArrayLibrary.Array_Length` _keys) 1)))))
  (bind _aswbp_enemy_actions_2 (cast `/Game/Blueprints/Widgets/WBP_EnemyActions` (`WidgetComponent.GetUserWidgetObject` (`self.Widget`))))
  (for (_array_element _array_index) (`self.ActionsForTurn`)
    (`KismetSystemLibrary.PrintString` _array_element)
    (bind _returnvalue (`|CreateWidget` "/Game/Blueprints/Widgets/WBP_ActionType.WBP_ActionType_C"))
    (switch `string` _array_element
      (:`Attack`
        (bind _actionimage (`/Game/Blueprints/Widgets/WBP_ActionType.ActionImage` _returnvalue))
        (`Image.SetBrushFromAsset` _actionimage "/Game/Materials/speech_bubble_sword_Brush.speech_bubble_sword_Brush"))
      (:`Heal`
        (`Image.SetBrushFromAsset` _actionimage "/Game/Materials/speech_bubble_heal_Brush.speech_bubble_heal_Brush"))
      (:`Block`
        (`Image.SetBrushFromAsset` _actionimage "/Game/Materials/speech_bubble_sheild_Brush.speech_bubble_sheild_Brush")))
    (bind _returnvalue_2 (`UniformGridPanel.AddChildToUniformGrid` (`/Game/Blueprints/Widgets/WBP_EnemyActions.Actions` _aswbp_enemy_actions_2) _returnvalue 0 _array_index))
    (`UniformGridSlot.SetHorizontalAlignment` _returnvalue_2 "HAlign_Fill")
    (`UniformGridSlot.SetVerticalAlignment` _returnvalue_2 "VAlign_Fill"))
  (`WidgetComponent.RequestRedraw` (`self.Widget`)))

(fn `InitializeEnemy`
  (bind _outrownames (`DataTableFunctionLibrary.GetDataTableRowNames` "/Game/Blueprints/DataTables/DT_EnemyInfo.DT_EnemyInfo"))
  (bind _returnvalue (`|GetDataTableRow` "/Game/Blueprints/DataTables/DT_EnemyInfo.DT_EnemyInfo" (`|GetArrayItem` _outrownames (`KismetMathLibrary.RandomInteger` (`KismetArrayLibrary.Array_Length` _outrownames))))
    (:`then`
      (bind (_enemyname _enemyhealth _armor _idleanimation _damagedanimation _deathanimation _attackanimation _blockanimation _healanimation _attack _defense _possibleactions) (break `/Game/Blueprints/DataTables/F_EnemyInfoStructure` _returnvalue))
      (`PaperFlipbookComponent.SetFlipbook` (`self.EnemySprite`) _idleanimation)
      (set `self.Name` _enemyname)
      (bind _output_get (set `self.CurrentHealth` _enemyhealth))
      (set `self.MaxHealth` _output_get)
      (set `self.Armor` _armor)
      (set `self.Attack` _attack)
      (set `self.Defense` _defense)
      (set `self.IdleFlipbook` _idleanimation)
      (set `self.DamagedFlipbook` _damagedanimation)
      (set `self.DeathFlipbook` _deathanimation)
      (set `self.AttackFlipbook` _attackanimation)
      (set `self.BlockFlipbook` _blockanimation)
      (set `self.HealFlipbook` _healanimation)
      (set `self.Actions` _possibleactions))))

(fn `ResetAnimation`
  (`PaperFlipbookComponent.SetFlipbook` (`self.EnemySprite`) (`self.IdleFlipbook`)))

(fn `TakeEnemyTurn`
  (bind _actionsforturn (`self.ActionsForTurn`))
  (if (<= (`self.CurrentHealth`) 0)
    (`self.AnimStateMachine`)
    (else
      (set `self.EnemyTakeAction` true)
      (if (`KismetArrayLibrary.Array_IsValidIndex` _actionsforturn)
        (`self.ApplyCardEffect` (`|GetArrayItem` _actionsforturn))
        (bind _aswbp_enemy_actions (cast `/Game/Blueprints/Widgets/WBP_EnemyActions` (`WidgetComponent.GetUserWidgetObject` (`self.Widget`))))
        (bind _actions (`/Game/Blueprints/Widgets/WBP_EnemyActions.Actions` _aswbp_enemy_actions))
        (cast `/Game/Blueprints/Widgets/WBP_ActionType` (`PanelWidget.GetChildAt` _actions 0))
        (`PanelWidget.RemoveChildAt` _actions 0)
        (`KismetArrayLibrary.Array_Remove` (`self.ActionsForTurn`))
        (`WidgetComponent.RequestRedraw` (`self.Widget`))))))

(fn `UserConstructionScript`)