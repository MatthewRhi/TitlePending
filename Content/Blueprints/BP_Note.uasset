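; BP_Note is a moving gameplay note with a left, right or both type, which DisplayType shows through the cylinder's material.
; EvaluateExpectation checks the pressed side while the note is destructible, latching both sides for both-type notes, then reports its Card to the player controller and fires OnPlayed.
; OnPlayed halts the projectile movement and chains grow and shrink timelines before destroying the actor.
; The controller's EnemyDead event also halts the note.
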(event `self.ReceiveBeginPlay`
  (add `self.OnPlayed` (delegate `PulseNote`))
  (bind _asbp_gameplay_phase_player_controller (cast `/Game/Blueprints/BP_GameplayPhase_PlayerController` (`GameplayStatics.GetPlayerController` 0)))
  (add `/Game/Blueprints/BP_GameplayPhase_PlayerController.EnemyDead` _asbp_gameplay_phase_player_controller (delegate `OnEnemyDead`)))

(event `PulseNote`
  (bind (_returnvalue_location _returnvalue_rotation _returnvalue_scale) (`KismetMathLibrary.BreakTransform` (`self.GetTransform`)))
  (bind (_returnvalue_location_2 _returnvalue_rotation_2 _returnvalue_scale_2) (`KismetMathLibrary.BreakTransform` (`self.GetTransform`)))
  (`ProjectileMovementComponent.SetVelocityInLocalSpace` (`self.ProjectileMovement`) (0.0 0.0 0.0))
  (bind (_direction _pulseline) (`Timeline|GrowTimeline` :!via `PlayFromStart`)
    (:`Update`
      (`self.K2_SetActorTransform` (`KismetMathLibrary.MakeTransform` _returnvalue_location _returnvalue_rotation (`KismetMathLibrary.VLerp` _returnvalue_scale (1.1 1.1 0.2) _pulseline))))
    (:`Finished`
      (bind (_direction_2 _shrinkline) (`Timeline|ShrinkTimeline` :!via `PlayFromStart`)
        (:`Update`
          (`self.K2_SetActorTransform` (`KismetMathLibrary.MakeTransform` _returnvalue_location_2 _returnvalue_rotation_2 (`KismetMathLibrary.VLerp` _returnvalue_scale_2 (0.5 0.5 0.0) _shrinkline))))
        (:`Finished`
          (`self.K2_DestroyActor`))))))

(event `OnEnemyDead`
  (`ProjectileMovementComponent.SetVelocityInLocalSpace` (`self.ProjectileMovement`) (0.0 0.0 0.0)))

(fn `DisplayType`
  (bind _cylinder (`self.Cylinder`))
  (switch `string` (`self.Type`)
    (:`L`
      (`PrimitiveComponent.SetMaterial` _cylinder 0 "/Game/Materials/M_LeftNote.M_LeftNote"))
    (:`R`
      (`PrimitiveComponent.SetMaterial` _cylinder 0 "/Game/Materials/M_RightNote.M_RightNote"))
    (:`B`
      (`PrimitiveComponent.SetMaterial` _cylinder 0 "/Game/Materials/M_BothNotes.M_BothNotes"))))

(fn `EvaluateExpectation`
  (params (Side :type String))
  (locals (BtnSide :type String))
  (set `local.BtnSide` Side)
  (switch `string` (`self.Type`)
    (:`Default`
      (if (and (`self.Destructible`) (`KismetStringLibrary.EqualEqual_StrStr` (`self.Type`) (`local.BtnSide`)))
        (bind _asbp_gameplay_phase_player_controller (cast `/Game/Blueprints/BP_GameplayPhase_PlayerController` (`GameplayStatics.GetPlayerController` 0) :!label _label))
        (`/Game/Blueprints/BP_GameplayPhase_PlayerController.NotePlayed` _asbp_gameplay_phase_player_controller (`self.Card`) "None")
        (`self.OnPlayed`)))
    (:`B`
      (switch `string` (`local.BtnSide`)
        (:`L`
          (bind _output_get (set `self.LeftRcvd` true)))
        (:`R`
          (bind _output_get_2 (set `self.RightRcvd` true))))
      (if (and _output_get _output_get_2 (`self.Destructible`))
        (goto _label)))))

(fn `UserConstructionScript`)